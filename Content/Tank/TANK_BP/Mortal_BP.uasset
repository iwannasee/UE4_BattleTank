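; Mortal_BP is a tank-game Blueprint with an aimed turret and barrel and a health bar widget.
; On BeginPlay it initialises the MortalAiming component with its turret and barrel, then casts the widget component's user widget to HealthBar and caches it.
; Every Tick pushes the current health percentage into that widget by polling rather than reacting to damage events.
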(event `self.ReceiveBeginPlay`
  (`TankAimingComponent.AimingInitialise` (`self.MortalAiming`) (`self.TankTurret`) (`self.TankBarrel`))
  (bind _ashealth_bar (cast `/Game/Tank/TANK_BP/HealthBar` (`WidgetComponent.GetUserWidgetObject` (`self.Widget`))))
  (bind _output_get (set `self.Health Bar` _ashealth_bar))
  (set `/Game/Tank/TANK_BP/HealthBar.Health Percent` (`self.GetHealthPercentage` self) _output_get))

(event `self.ReceiveTick`
  (params (DeltaSeconds :type "Float (single-precision)"))
  (set `/Game/Tank/TANK_BP/HealthBar.Health Percent` (`self.GetHealthPercentage` self) (`self.Health Bar`)))

(fn `UserConstructionScript`)