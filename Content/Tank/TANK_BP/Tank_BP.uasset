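; Player tank pawn that wires input to aiming, movement and camera components and shows its health on a widget bar.
; BeginPlay hands the turret and barrel to TankAiming and both tracks to TankMovement, then caches the HealthBar widget, which Tick updates with the health percentage.
; Input axes rotate the azimuth and spring arm, drive movement intents and pitch the barrel directly, while actions fire and toggle first/third-person views.
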(event `self.ReceiveBeginPlay`
  (`TankAimingComponent.AimingInitialise` (`self.TankAiming`) (`self.TankTurret`) (`self.TankBarrel`))
  (`TankMovementComponent.Initialise` (`self.TankMovement`) (`self.TankTrack_L`) (`self.TankTrack_R`))
  (bind _ashealth_bar (cast `/Game/Tank/TANK_BP/HealthBar` (`WidgetComponent.GetUserWidgetObject` (`self.Widget`))))
  (set `self.HealthBar` _ashealth_bar)
  (set `/Game/Tank/TANK_BP/HealthBar.Health Percent` (`self.GetHealthPercentage` self) _ashealth_bar))

(event `self.ReceiveTick`
  (params (DeltaSeconds :type "Float (single-precision)"))
  (set `/Game/Tank/TANK_BP/HealthBar.Health Percent` (`self.GetHealthPercentage` self) (`self.HealthBar`)))

(event `InputAction|FirstPerson`
  (params (Key :type "Key Structure"))
  (:`Pressed`
    (`ActorComponent.ToggleActive` (`self.1st`))
    (`ActorComponent.ToggleActive` (`self.3rd`))))

(event `InputAxis|AimAzimuth`
  (params (AxisValue :type "Float (single-precision)"))
  ;[1 1 1] Camera Input Binding
  (`SceneComponent.K2_AddLocalRotation` (`self.Azimuth`) (`KismetMathLibrary.MakeRotator` 0.0 0.0 AxisValue) false false))

(event `InputAxis|AimElevation`
  (params (AxisValue :type "Float (single-precision)"))
  ;[1 1 1] Camera Input Binding
  (`SceneComponent.K2_AddLocalRotation` (`self.SpringArm`) (`KismetMathLibrary.MakeRotator` 0.0 AxisValue) false false))

(event `InputAxis|MoveForward`
  (params (AxisValue :type "Float (single-precision)"))
  ;[1 1 1] Movement Input Binding
  (`TankMovementComponent.IntendMoveForward` (`self.TankMovement`) AxisValue))

(event `InputAxis|Turn Right`
  (params (AxisValue :type "Float (single-precision)"))
  ;[1 1 1] Movement Input Binding
  (`TankMovementComponent.IntendTurnRight` (`self.TankMovement`) AxisValue))

(event `InputAxis|RaiseBarrel`
  (params (AxisValue :type "Float (single-precision)"))
  ;[1 1 1] Barrel Input Binding
  (`SceneComponent.K2_AddLocalRotation` (`self.TankBarrel`) (`KismetMathLibrary.MakeRotator` 0.0 AxisValue) false false))

(event `InputAction|Fire`
  (params (Key :type "Key Structure"))
  ;[1 1 1] Barrel Input Binding
  (:`Pressed`
    (`TankAimingComponent.Fire` (`self.TankAiming`))))

(fn `UserConstructionScript`)